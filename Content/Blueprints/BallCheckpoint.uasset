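; Checkpoint actor for a ball that shows a success message and teleports any overlapping actor, while its mesh root spins on Tick.
; On overlap it deactivates every BP_FallingTrigger, waits briefly, then moves the actor to TeleportLocation, an offset rotated into the checkpoint's orientation.
; After another short delay it clears the text and reactivates all those triggers.
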(event EventBeginPlay)

(event EventTick
  (params (DeltaSeconds :type Float%20%28single-precision%29))
  (Transformation|AddLocalRotation (Variables|Default|GetMeshRoot) (Class|KismetMathLibrary|MakeRot (* DeltaSeconds 1e+02) 0.0 0.0) false))

(event EventActorBeginOverlap
  (params (OtherActor :type Actor%20Object%20Reference))
  (Rendering|Components|TextRender|SetText (Variables|Default|GetSuccessText) "Success!!")
  (bind _outactors (Actor|GetAllActorsOfClass "/Game/Blueprints/BP_FallingTrigger.BP_FallingTrigger_C"))
  (for _array_element _outactors
    (Variables|/Game/Blueprints/BP_FallingTrigger.BP_FallingTrigger_C|SetActive _array_element false))
  (Utilities|FlowControl|Delay 1.0)
  (Transformation|SetActorLocation OtherActor (+ (Transformation|GetWorldLocation) (Math|Vector|RotateVector (Variables|Default|GetTeleport%20Location) (Transformation|GetWorldRotation))) false)
  (Utilities|FlowControl|Delay 0.2)
  (Rendering|Components|TextRender|SetText "")
  (for _array_element_2 _outactors
    (Variables|/Game/Blueprints/BP_FallingTrigger.BP_FallingTrigger_C|SetActive _array_element_2 true)))

(fn ConstructionScript)